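; Zombie enemy for a wave-based game that chases and attacks the player and pays out money when damaged.
; ChasePlayer re-invokes itself around AI MoveTo, dealing damage at close range, gated by a delayed attack cooldown.
; DealDamage awards money per hit; death ragdolls the mesh, rewards the kill and destroys the actor after a delay.
; Deaths also update the wave count on the game manager, whose reference comes from Player_BP.
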(event `RechargeAttack`
  ;[1 1 1] Attack cooldown
  (`KismetSystemLibrary.Delay` (`self.AttackRate`))
  (set `self.CanAttack` true))

(event `Chase Player`
  ;[1 1 1] Chase and attack player
  (if (not (`self.EnemyDied`))
    (`|AIMoveTo` self (0.0 0.0 0.0) (`GameplayStatics.GetPlayerCharacter` 0) 50.0
      (:`OnSuccess`
        (if (`self.CanAttack`)
          (set `self.CanAttack` false)
          (`self.RechargeAttack`)
          (`self.Chase Player`)
          (if (`self.EnemyDied`)
            _
            (elif (<= (`self.GetDistanceTo` self (`GameplayStatics.GetPlayerCharacter` 0)) 75.0)
              (bind _asplayer_bp (cast `/Game/ZombieCreed_Game/Characters/Player_Character/Player_BP` (`GameplayStatics.GetPlayerCharacter` 0)))
              (`/Game/ZombieCreed_Game/Characters/Player_Character/Player_BP.Take Damage` _asplayer_bp (`self.Damage`))
              (else
                (`self.Chase Player`))))
          (else
            (`self.Chase Player`))))
      (:`OnFail`
        (`self.Chase Player`)))))

(event `self.ReceiveBeginPlay`
  ;[1 1 1] Chase player until player or enemy die - get the gamemanager bp
  (set `self.Health` (`self.MaxHealth`))
  (bind _asplayer_bp (cast `/Game/ZombieCreed_Game/Characters/Player_Character/Player_BP` (`GameplayStatics.GetPlayerCharacter` 0)))
  (set `self.GM_REF` (`/Game/ZombieCreed_Game/Characters/Player_Character/Player_BP.GM_REF` _asplayer_bp))
  (`KismetSystemLibrary.Delay` 0.2)
  (`self.Chase Player`))

(event `Deal Damage`
  (params (Damage :type "Float (double-precision)"))
  (bind _gm_ref (`self.GM_REF`))
  ;[1 1 1] Deal damage to zombie
  (bind _output_get (set `self.Health` (- (`self.Health`) Damage)))
  (if (<= _output_get 0.0)
    (`PrimitiveComponent.SetSimulatePhysics` (`self.Mesh`) true)
    (if (not (`self.EnemyDied`))
      (bind _asplayer_bp (cast `/Game/ZombieCreed_Game/Characters/Player_Character/Player_BP` (`GameplayStatics.GetPlayerCharacter` 0)))
      (set `/Game/ZombieCreed_Game/Characters/Player_Character/Player_BP.Money` (+ (`/Game/ZombieCreed_Game/Characters/Player_Character/Player_BP.Money` _asplayer_bp) (`self.KillValue`)) _asplayer_bp)
      (`/Game/ZombieCreed_Game/Characters/Player_Character/Player_BP.IncrementKillCount` _asplayer_bp)
      (set `self.EnemyDied` true)
      (bind _result (`/Engine/EditorBlueprintResources/StandardMacros.DecrementInt` (`/Game/ZombieCreed_Game/Blueprints/GameManager_BP.ZombieLeftInWave` _gm_ref))
        (:`  `
          (set `/Game/ZombieCreed_Game/Blueprints/GameManager_BP.ZombieLeftInWave` _result _gm_ref)
          (`/Game/ZombieCreed_Game/Blueprints/GameManager_BP.CheckForNextWave` _gm_ref)
          (`KismetSystemLibrary.Delay` 1.0)
          (`self.K2_DestroyActor`))))
    (else
      ;[1 1 1] Add money on hit
      (bind _asplayer_bp_2 (cast `/Game/ZombieCreed_Game/Characters/Player_Character/Player_BP` (`GameplayStatics.GetPlayerCharacter` 0)))
      (set `/Game/ZombieCreed_Game/Characters/Player_Character/Player_BP.Money` (+ (`/Game/ZombieCreed_Game/Characters/Player_Character/Player_BP.Money` _asplayer_bp_2) (`self.HitValue`)) _asplayer_bp_2))))

(fn `UserConstructionScript`)
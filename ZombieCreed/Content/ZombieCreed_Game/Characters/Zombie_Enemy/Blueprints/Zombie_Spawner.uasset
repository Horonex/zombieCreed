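; Zombie spawner behind a five-plank barricade that spawns enemies while the game manager, fetched via Player_BP, has spawn weight left.
; A Delay on Tick paces attempts, each removing a repair point through Repair, which also updates plank visibility.
; Once repairs drop below one, attempts spend weight and randomly spawn normal or boss zombies.
; The small variant is unreachable because RandomInteger(2) never returns 2.
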(event `self.ReceiveTick`
  (params (DeltaSeconds :type "Float (single-precision)"))
  (bind _returnvalue (`KismetMathLibrary.RandomInteger` 2))
  (bind _weightlefttospawn (`/Game/ZombieCreed_Game/Blueprints/GameManager_BP.WeightLeftToSpawn` (`self.GM_REF`)))
  (bind _location (.location (`SceneComponent.K2_GetComponentToWorld` (`self.Scene`))))
  (bind _rotation (.rotation (`SceneComponent.K2_GetComponentToWorld` (`self.Scene`))))
  ;[1 1 1] Spawn zombies
  (`KismetSystemLibrary.Delay` (`self.SpawnRate`))
  (if (> _weightlefttospawn 0)
    (bind _canspawn (`self.trySpawn` 1))
    (if _canspawn
      (bind _result (`/Engine/EditorBlueprintResources/StandardMacros.DecrementInt` _weightlefttospawn)
        (:`  `
          (set `/Game/ZombieCreed_Game/Blueprints/GameManager_BP.WeightLeftToSpawn` _result (`self.GM_REF`))
          (if (== _returnvalue 0)
            (`AIBlueprintHelperLibrary.SpawnAIFromClass` "/Game/ZombieCreed_Game/Characters/Zombie_Enemy/Blueprints/Zombie_BP.Zombie_BP_C" null _location _rotation)
            (elif (== _returnvalue 1)
              (`AIBlueprintHelperLibrary.SpawnAIFromClass` "/Game/ZombieCreed_Game/Characters/Zombie_Enemy/Blueprints/Zombie_BP_Boss.Zombie_BP_Boss_C" null _location _rotation)
              (elif (== _returnvalue 2)
                (`AIBlueprintHelperLibrary.SpawnAIFromClass` "/Game/ZombieCreed_Game/Characters/Zombie_Enemy/Blueprints/Zombie_BP_Small.Zombie_BP_Small_C" null _location _rotation)))))))))

(event `self.ReceiveBeginPlay`
  ;[1 1 1] Get reference to GameManager
  (`KismetSystemLibrary.Delay` 2.0)
  (bind _asplayer_bp (cast `/Game/ZombieCreed_Game/Characters/Player_Character/Player_BP` (`GameplayStatics.GetPlayerCharacter` 0)))
  (set `self.GM_REF` (`/Game/ZombieCreed_Game/Characters/Player_Character/Player_BP.GM_REF` _asplayer_bp)))

(fn `Repair`
  (params (repairValue :type Integer))
  (bind _repairs (`self.repairs`))
  (set `self.repairs` (+ (`self.repairs`) repairValue))
  (`|ExecutionSequence`
    (:`then_0`
      (`SceneComponent.SetVisibility` (`self.plank1`) (>= _repairs 1) false))
    (:`then_1`
      (`SceneComponent.SetVisibility` (`self.plank2`) (>= _repairs 2) false))
    (:`then_2`
      (`SceneComponent.SetVisibility` (`self.plank3`) (>= _repairs 3) false))
    (:`then_3`
      (`SceneComponent.SetVisibility` (`self.plank4`) (>= _repairs 4) false))
    (:`then_4`
      (`SceneComponent.SetVisibility` (`self.plank5`) (>= _repairs 5) false))))

(fn `trySpawn`
  (params (Weight :type Integer :default 1))
  (returns (canSpawn :type Boolean))
  (`self.Repair` (* Weight -1))
  (return (< (`self.repairs`) 1)))

(fn `UserConstructionScript`)